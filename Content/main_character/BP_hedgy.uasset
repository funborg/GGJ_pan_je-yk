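; Player hedgehog character with a flipbook sprite that toggles between walking and a physics-driven rolling ball.
; Rolling applies camera-relative angular impulses and picks up tagged BP_item_base actors onto ItemsRotation.
; Tick fakes the roll by keeping the capsule upright, spinning attached items from velocity and scaling flipbook speed.
; Mid-air jump triggers a ground pound that detaches items on landing, while WIP interaction passes the attached list to BPI_dialogue actors.
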(event OnComponentBeginOverlap(CapsuleComponent)
  (params (OverlappedComponent :type Primitive%20Component%20Object%20Reference) (OtherActor :type Actor%20Object%20Reference) (OtherComp :type Primitive%20Component%20Object%20Reference) (OtherBodyIndex :type Integer) (bFromSweep :type Boolean) (SweepResult :type Hit%20Result%20Structure%20%28by%20ref%29))
  ;[1 1 1] podniesienie przedmiotu
  (if (Variables|Default|Getis%20rolling)
    (bind _asbp_item_base (Utilities|Casting|CastToBP_item_base OtherActor))
    (if (Actor|ActorHasTag OtherActor "canBePicked")
      (Default|OnAttached _asbp_item_base (Transformation|GetWorldLocation (Variables|Collision|GetCapsuleComponent)))
      (Transformation|AttachComponentToComponent _asbp_item_base (Variables|Default|Getitems%20rotation) "None" "KeepWorld" "KeepWorld" "KeepWorld" true)
      (Utilities|Array|Add (Variables|Default|Getattached%20actors) _asbp_item_base)
      (Audio|PlaySound2D "/Game/sounds/leaves/leaves_01_Cue.leaves_01_Cue" 1.0 1.0 0.0 0 0))))

(event Input|EnhancedActionEvents|EnhancedInputActionIA_move
  (params (ActionValue :type Vector%202D%20Structure) (ElapsedSeconds :type Float%20%28double-precision%29) (TriggeredSeconds :type Float%20%28double-precision%29) (InputAction :type Input%20Action%20Object%20Reference :default "/Game/main_character/Input/IA_move.IA_move"))
  (bind _returnvalue (Transformation|GetVelocity))
  (bind _returnvalue_2 (Pawn|GetControlRotation :!class /Script/Engine.Pawn))
  (bind _returnvalue_3 (Pawn|GetControlRotation :!class /Script/Engine.Pawn))
  (bind _maximum_vel (Variables|Default|Getmaximum%20vel))
  (bind _maximum_vel_2 (Variables|Default|Getmaximum%20vel))
  (bind _returnvalue_4 (Math|Vector|GetForwardVector (Math|Rotator|MakeRotator (.roll _returnvalue_2) 0.0 (.yaw _returnvalue_2))))
  (bind _returnvalue_5 (Math|Vector|GetRightVector (Math|Rotator|MakeRotator (.roll _returnvalue_3) 0.0 (.yaw _returnvalue_3))))
  ;[1 1 1] poruszanie się postacią
  ;;[1 1 1] tryb kulki
  (if (Variables|Default|Getis%20rolling)
    (if (> (.y ActionValue) 0.0)
      (if (> (.y _returnvalue) _maximum_vel_2)
        _
        (else
          (Class|PrimitiveComponent|AddAngularImpulseinDegrees (Variables|Collision|GetCapsuleComponent) (* _returnvalue_4 (.y ActionValue) (Variables|Default|Getrolling%20speed) -1.0) "None" true :!label _label)))
      (elif (< (.y _returnvalue) (* _maximum_vel_2 -1.0))
        _
        (else
          (goto _label))))
    (if (> (.x ActionValue) 0.0)
      (if (not (> (.x _returnvalue) _maximum_vel))
        (Class|PrimitiveComponent|AddAngularImpulseinDegrees (Variables|Collision|GetCapsuleComponent) (* _returnvalue_5 (.x ActionValue) (Variables|Default|Getrolling%20speed)) "None" true :!label _label_2)
        (Audio|PlaySound2D "/Game/sounds/roll/applepie_roll_01_Cue.applepie_roll_01_Cue" 1.0 1.0 0.0 "/Game/sounds/roll/Roll_SoundConcurrency.Roll_SoundConcurrency" 0))
      (elif (not (< (.x _returnvalue) (* _maximum_vel -1.0)))
        (goto _label_2)))
    (else
      ;;[1 1 1] chodzenie
      (Pawn|Input|AddMovementInput _returnvalue_4 (.x ActionValue) false)
      (Pawn|Input|AddMovementInput _returnvalue_5 (.y ActionValue) false)
      (if (!= (.y ActionValue) 0.0)
        (Transformation|SetWorldRotation (Variables|Default|Getsprite) (Math|Rotator|MakeRotator 0.0 0.0 (Math|Float|SelectFloat -9e+01 9e+01 (< (.y ActionValue) 0.0))) false false)))))

(event Input|EnhancedActionEvents|EnhancedInputActionIA_mode_switch
  (params (ActionValue :type Boolean) (ElapsedSeconds :type Float%20%28double-precision%29) (TriggeredSeconds :type Float%20%28double-precision%29) (InputAction :type Input%20Action%20Object%20Reference :default "/Game/main_character/Input/IA_mode_switch.IA_mode_switch"))
  ;[1 1 1] zmiana trybu
  (:Started
    (if (not (AI|Components|NavMovement|IsFalling (Variables|Character|GetCharacterMovement)))
      (bind _output_get (Variables|Default|Setis%20rolling (not (Variables|Default|Getis%20rolling))))
      (Physics|SetSimulatePhysics (Variables|Collision|GetCapsuleComponent) _output_get)
      (Sprite|SetFlipbook (Variables|Default|Getsprite) (select _output_get "/Game/textures/main_character/ballin_mode/Kulka.Kulka" "/Game/textures/main_character/idle/idle.idle"))
      (Transformation|SetWorldTransform (Variables|Collision|GetCapsuleComponent) (Math|Transform|MakeTransform (+ (Transformation|GetActorLocation) "0.000000,0.000000,30.000000") "0, 0, 0" "1.000000,1.000000,1.000000") false false)
      (Components|Timeline|SetPlayRate (Variables|Default|Getsprite) 1.0))))

(event Input|EnhancedActionEvents|EnhancedInputActionIA_jump
  (params (ActionValue :type Boolean) (ElapsedSeconds :type Float%20%28double-precision%29) (TriggeredSeconds :type Float%20%28double-precision%29) (InputAction :type Input%20Action%20Object%20Reference :default "/Game/main_character/Input/IA_jump.IA_jump"))
  ;[1 1 1] skok
  (:Started
    (if (not (Variables|Default|Getis%20rolling))
      (Character|Jump)
      ;;[1 1 1] ground pound
      (Audio|PlaySound2D "/Game/sounds/jumps/Random_Jump.Random_Jump" 1.0 1.0 0.0 0 0)
      (if (AI|Components|NavMovement|IsFalling (Variables|Character|GetCharacterMovement))
        (Variables|Default|SetGP%20ready true)
        (Sprite|SetFlipbook (Variables|Default|Getsprite) "/Game/textures/main_character/ballin_mode/Kulka.Kulka")
        (Physics|AddImpulse (Variables|Character|GetCharacterMovement) "0.000000,0.000000,-1500.000000" true)))))

(event Input|EnhancedActionEvents|EnhancedInputActionIA_interact
  (params (ActionValue :type Boolean) (ElapsedSeconds :type Float%20%28double-precision%29) (TriggeredSeconds :type Float%20%28double-precision%29) (InputAction :type Input%20Action%20Object%20Reference :default "/Game/main_character/Input/IA_interact.IA_interact"))
  ;[1 1 1] interakcja (WIP DO NOT TOUCH)
  (:Started
    (bind _array_element (Utilities|Array|ForEachLoopwithBreak (Collision|GetOverlappingActors "/Game/characters/BASE/bp_base_char.bp_base_char_C" :!class /Script/Engine.Actor))
      (:LoopBody
        (if (Utilities|DoesObjectImplementInterface _array_element "/Game/characters/BASE/BPI_dialogue.BPI_dialogue_C")
          (Class|BPIDialogue|Interact(Message) _array_element (Variables|Default|Getattached%20actors)))))))

(event Input|EnhancedActionEvents|EnhancedInputActionIA_move
  (params (ActionValue :type Vector%202D%20Structure) (ElapsedSeconds :type Float%20%28double-precision%29) (TriggeredSeconds :type Float%20%28double-precision%29) (InputAction :type Input%20Action%20Object%20Reference :default "/Game/main_character/Input/IA_move.IA_move"))
  (bind _sprite (Variables|Default|Getsprite))
  ;[1 1 1] zmiana animacji
  (:Triggered
    (if (not (or (Variables|Default|Getis%20rolling) (Variables|Default|GetGP%20ready))) :!label _label
      (if (and (== (.x ActionValue) 0.0) (== (.y ActionValue) 0.0))
        (Sprite|SetFlipbook _sprite "/Game/textures/main_character/idle/idle.idle")
        (else
          (if (> (.x ActionValue) 0.0)
            (Sprite|SetFlipbook _sprite "/Game/textures/main_character/walk_back/walk_back.walk_back")
            (else
              (Sprite|SetFlipbook _sprite "/Game/textures/main_character/walk/walk.walk")))
          (Audio|PlaySound2D "/Game/sounds/walk/applepie_walk_07_Cue.applepie_walk_07_Cue" 0.95 1.0 0.0 "/Game/sounds/walk/Walk_SoundConcurrency.Walk_SoundConcurrency" 0)))))
  (:Completed
    (goto _label)))

(event EventBeginPlay
  ;[1 1 1] dodanie mapowania kontroli
  (Audio|PlaySound2D "/Game/sounds/music/main_time_1_Cue.main_time_1_Cue" 1.0 1.0 0.0 0 0)
  (bind _asplayer_controller (Utilities|Casting|CastToPlayerController (Game|GetPlayerController 0)))
  (Input|AddMappingContext (PlayerController|LocalPlayerSubsystems|GetEnhancedInputLocalPlayerSubsystem _asplayer_controller) "/Game/main_character/Input/mapping.mapping" 0 "(bIgnoreAllPressedKeysUntilRelease=True,bForceImmediately=False,bNotifyUserSettings=False)"))

(event EventOnLanded
  (params (Hit :type Hit%20Result%20Structure%20%28by%20ref%29))
  ;[1 1 1] uderzenie ciałem w ziemie
  (if (Variables|Default|GetGP%20ready)
    (Variables|Default|SetGP%20ready false)
    (Sprite|SetFlipbook (Variables|Default|Getsprite) "/Game/textures/main_character/idle/idle.idle")
    (for _array_element (Variables|Default|Getattached%20actors)
      (Default|Detached _array_element)
      (Audio|PlaySound2D "/Game/sounds/swoosh/swoosh_01_Cue.swoosh_01_Cue" 1.0 1.0 0.0 0 _array_element))))

(event EventTick
  (params (DeltaSeconds :type Float%20%28single-precision%29))
  (bind _returnvalue (Transformation|GetVelocity))
  ;[1 1 1] obracanie przedmiotu w ruchu
  (if (Variables|Default|Getis%20rolling)
    (Transformation|AddWorldRotation (Variables|Default|Getitems%20rotation) (Math|Rotator|MakeRotator (* (.y _returnvalue) DeltaSeconds) (* (* (.x _returnvalue) DeltaSeconds) -1.0) 0.0) false false)
    (Transformation|SetWorldRotation (Variables|Collision|GetCapsuleComponent) "0, 0, 0" false false)
    (Components|Timeline|SetPlayRate (Variables|Default|Getsprite) (+ (/ (Class|KismetMathLibrary|GetMax2D (Math|Vector2D|MakeVector2D (Math|Float|Absolute(Float) (.x _returnvalue)) (Math|Float|Absolute(Float) (.y _returnvalue)))) (Variables|Default|Getrolling%20speed)) 1.0))))

(fn ConstructionScript)