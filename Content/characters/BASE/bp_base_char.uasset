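; Base quest NPC that runs a branching-by-state dialogue and takes delivery of a requested item from the player hedgehog.
; Construction loads sprite, item ID and five dialogue sets from the Character_data row matching its Name.
; Interact detaches a matching carried item during an active quest, marks it delivered, then drives the text box.
; Finishing a dialogue set advances the quest state; a pickup-capable actor leaving overlap resets dialogue.
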(event Custom|dialouge%20finished
  ;[1 1 1] dialog z npcem
  (Math|Integer|IncrementInt (Variables|Default|Getdialogue%20index)))

(event Custom|Progress%20Dialogue
  ;[1 1 1] dialog z npcem
  (if (< (Variables|Default|Getdialogue%20index) (Utilities|Array|Length (Utilities|Select :Index (Variables|Default|Getquest%20state) :NewEnumerator0 (Variables|Default|Getpre%20quest%20dialouge) :NewEnumerator1 (Variables|Default|Getquest%20giving%20dialouge) :NewEnumerator2 (Variables|Default|Getongoing%20quest%20dialogue%20set) :NewEnumerator4 (Variables|Default|Getquest%20completion%20dialouge) :NewEnumerator3 (Variables|Default|Getpost%20quest%20dialouge))))
    ;;[1 1 1] twórz text box ja go niema
    (Utilities|IsValid (Variables|Default|Getdiag%20box)
      (:Is%20Valid
        _)
      (:Is%20Not%20Valid
        (bind _returnvalue (UserInterface|CreateWidget "/Game/characters/BASE/WB_diagBox.WB_diagBox_C" (Game|GetPlayerController 0)))
        (bind _output_get (Variables|Default|Setdiag%20box _returnvalue))
        (UserInterface|Viewport|AddtoViewport _output_get 0)))
    (Rendering|Components|TextRender|SetText (Variables|/Game/characters/BASE/WB_diagBox.WB_diagBox_C|Getnametext (Variables|Default|Getdiag%20box)) (Utilities|Text|ToText(Name) (select (.ismcspeaking (Utilities|Array|Get(acopy) (Utilities|Select :Index (Variables|Default|Getquest%20state) :NewEnumerator0 (Variables|Default|Getpre%20quest%20dialouge) :NewEnumerator1 (Variables|Default|Getquest%20giving%20dialouge) :NewEnumerator2 (Variables|Default|Getongoing%20quest%20dialogue%20set) :NewEnumerator4 (Variables|Default|Getquest%20completion%20dialouge) :NewEnumerator3 (Variables|Default|Getpost%20quest%20dialouge)) (Variables|Default|Getdialogue%20index))) "mr.hedgehog" (Variables|Components|Getname))))
    (Default|StartReadingDialouge (Variables|Default|Getdiag%20box) (.dialouge (Utilities|Array|Get(acopy) (Utilities|Select :Index (Variables|Default|Getquest%20state) :NewEnumerator0 (Variables|Default|Getpre%20quest%20dialouge) :NewEnumerator1 (Variables|Default|Getquest%20giving%20dialouge) :NewEnumerator2 (Variables|Default|Getongoing%20quest%20dialogue%20set) :NewEnumerator4 (Variables|Default|Getquest%20completion%20dialouge) :NewEnumerator3 (Variables|Default|Getpost%20quest%20dialouge)) (Variables|Default|Getdialogue%20index))) self)
    (else
      ;;[1 1 1] zamknięcie dialogu
      (Variables|Default|Setquest%20state (Utilities|Select :Index (Variables|Default|Getquest%20state) :NewEnumerator0 "NewEnumerator0" :NewEnumerator1 "NewEnumerator2" :NewEnumerator2 "NewEnumerator2" :NewEnumerator4 "NewEnumerator3" :NewEnumerator3 "NewEnumerator3"))
      (Variables|Default|Setdialogue%20index 0)
      (Widget|RemovefromParent (Variables|Default|Getdiag%20box))
      (Variables|Default|Setdiag%20box 0)
      (Utilities|Platform|CollectGarbage))))

(event EventBeginPlay
  (Variables|Default|Setquest%20state "NewEnumerator1"))

(event Collision|EventActorBeginOverlap
  (params (OtherActor :type Actor%20Object%20Reference)))

(event EventTick
  (params (DeltaSeconds :type Float%20%28single-precision%29)))

(event EventInteract
  (params (NewParam :type Array%20of%20BP%20Item%20Base%20Object%20References))
  ;[1 1 1] dostawa itemów (do wywalenia za
  (if (Utilities|Enum|Equal(Enum) (Variables|Default|Getquest%20state) "NewEnumerator2")
    (bind _array_element (Utilities|Array|ForEachLoopwithBreak NewParam :!label _label)
      (:LoopBody
        (if (== (.id (Variables|/Game/items/BP_item_base.BP_item_base_C|Getitem_type _array_element)) (Variables|Default|Getitem%20needed%20ID))
          (Transformation|DetachFromActor _array_element "KeepRelative" "KeepRelative" "KeepRelative")
          (Default|Detached _array_element)
          (bind _asbp_hedgy (Utilities|Casting|CastToBP_hedgy (Game|GetPlayerCharacter 0)))
          (Utilities|Array|RemoveItem (Variables|/Game/main_character/BP_hedgy.BP_hedgy_C|Getattached%20actors _asbp_hedgy) _array_element)
          (Utilities|Array|RemoveItem (Variables|/Script/Engine.Actor|GetTags _array_element) "canBePicked")
          (Transformation|SetWorldLocation (Variables|/Game/items/BP_item_base.BP_item_base_C|Getphysics%20hitbox _array_element) (+ (Transformation|GetWorldLocation (Variables|Collision|GetCapsuleComponent)) "50.000000,50.000000,50.000000") false true)
          (Variables|Default|Setquest%20state "NewEnumerator4")
          (goto _label Break)))
      (:Completed
        (CallFunction|ProgressDialogue :!label _label_2)))
    (else
      (goto _label_2))))

(event Collision|EventActorEndOverlap
  (params (OtherActor :type Actor%20Object%20Reference))
  ;[1 1 1] dialog z npcem
  ;;[1 1 1] zamknięcie dialogu
  (if (Utilities|DoesObjectImplementInterface OtherActor "/Game/main_character/BPI_pickup.BPI_pickup_C")
    (Variables|Default|Setdialogue%20index 0)
    (Widget|RemovefromParent (Variables|Default|Getdiag%20box))
    (Variables|Default|Setdiag%20box 0)
    (Utilities|Platform|CollectGarbage)))

(fn ConstructionScript
  (bind _returnvalue (Utilities|GetDataTableRow "/Game/characters/BASE/character_data.character_data" (Variables|Components|Getname))
    (:then
      (Sprite|SetFlipbook (Variables|Default|GetPaperFlipbook) (.sprite _returnvalue))
      (Variables|Default|Setitem%20needed%20ID (.quest_id _returnvalue))
      (Variables|Default|Setpre%20quest%20dialouge (.prequestdialouge _returnvalue))
      (Variables|Default|Setquest%20giving%20dialouge (.questgivingdialouge _returnvalue))
      (Variables|Default|Setongoing%20quest%20dialogue%20set (.ongoingquestdialogueset _returnvalue))
      (Variables|Default|Setquest%20completion%20dialouge (.questcompletiondialouge _returnvalue))
      (Variables|Default|Setpost%20quest%20dialouge (.postquestdialouge _returnvalue)))))