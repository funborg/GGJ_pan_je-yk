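; Decor volume that scatters leaf items throughout a box when play begins.
; The construction script sizes the box from its InBoxExtent variable, and BeginPlay spawns BP_item_base actors at random offsets within those extents, in numbers proportional to the extent product.
; Each spawn gets a randomly selected leaf item data name; RandomInteger(2) only reaches the first two of the three options, so "lisc3" is never chosen.
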(event EventBeginPlay
  (bind _in_box_extent (Variables|Default|GetIn%20Box%20Extent))
  (for _index (range 0 (Math|Float|Round (/ (* (.x _in_box_extent) (.y _in_box_extent) (.z _in_box_extent)) 1e+05)))
    (Game|SpawnActorfromClass "/Game/items/BP_item_base.BP_item_base_C" (Math|Transform|MakeTransform (+ (Transformation|GetWorldLocation (Variables|Default|GetBox)) (Math|Vector|MakeVector (Math|Random|RandomFloatinRange (* (.x _in_box_extent) -1.0) (.x _in_box_extent)) (Math|Random|RandomFloatinRange (* (.y _in_box_extent) -1.0) (.y _in_box_extent)) (Math|Random|RandomFloatinRange (* (.z _in_box_extent) -1.0) (.z _in_box_extent)))) "0, 0, 0" "1.000000,1.000000,1.000000") "Undefined" "MultiplyWithRoot" 0 (Utilities|Select :Index (Math|Random|RandomInteger 2) :Option%200 "lisc1" :Option%201 "lisc2" :Option%202 "lisc3") 0)))

(fn ConstructionScript
  (Components|Box|SetBoxExtent (Variables|Default|GetBox) (Variables|Default|GetIn%20Box%20Extent) true))